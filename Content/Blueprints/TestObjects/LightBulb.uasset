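; LightBulb is a test object that changes its light color in response to a button message.
; RecieveButtonMsg compares the incoming Channel to its ButtonChannel and, on a match, sets the PointLight to a random color.
; The event graph and construction script are empty, and a leftover debug print is never executed.
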(event EventBeginPlay)

(event Collision|EventActorBeginOverlap
  (params (OtherActor :type Actor%20Object%20Reference)))

(event EventTick
  (params (DeltaSeconds :type Float%20%28single-precision%29)))

(fn ConstructionScript)

(fn RecieveButtonMsg
  (params (channel :type Integer))
  (bind _buttonchannel (Variables|Default|GetButtonChannel))
  (bind _returnvalue (== channel _buttonchannel))
  (if _returnvalue
    (bind _output_get (LocalVariables|SetNewLocalVar_0 (Utilities|Struct|MakeLinearColor (Math|Random|RandomFloatinRange 0.0 1.0) (Math|Random|RandomFloatinRange 0.0 1.0) (Math|Random|RandomFloatinRange 0.0 1.0) (Math|Random|RandomFloatinRange 0.0 1.0))))
    (Rendering|Components|Light|SetLightColor (Variables|Default|GetPointLight) _output_get true)
    (return _returnvalue)))