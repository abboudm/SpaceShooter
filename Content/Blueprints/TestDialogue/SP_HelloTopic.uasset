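; Test dialogue script for a Hello topic that visibly moves its Parent actor while it runs.
; StartScript raises the Parent by a fixed vertical offset and StopScript lowers it by the same amount, both with sweep enabled.
; IsActive reports true only while the Spoken flag is unset, so the topic is inactive once spoken.
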(event EventStopScript
  (bind _parent (Variables|Default|GetParent))
  (Transformation|SetActorLocation _parent (- (Transformation|GetActorLocation _parent) "0, 0,50.000000") true false))

(event EventStartScript
  (bind _parent (Variables|Default|GetParent))
  (Transformation|SetActorLocation _parent (+ (Transformation|GetActorLocation _parent) "0, 0,50.000000") true false))

(fn IsActive
  (return (not (Variables|Default|GetbSpoken))))